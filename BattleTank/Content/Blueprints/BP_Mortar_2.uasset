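; BP_Mortar_2 is a mortar turret actor with a health bar widget.
; On BeginPlay it initializes its MortarAiming component with the Barrel and Dome, the latter serving as the turret.
; It then casts the HealthBar component's user widget to WB_HealthBar and sets itself as that widget's TankRef.
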(event EventBeginPlay
  (Class|TankAimingComponent|Initialize (Variables|Default|GetMortarAiming) (Variables|Default|GetBarrel) (Variables|Default|GetDome))
  (CallFunction|InitializeHealthBarWidget))

(fn ConstructionScript)

(fn InitializeHealthBarWidget
  (bind _aswb_health_bar (Utilities|Casting|CastToWB_HealthBar (UserInterface|GetUserWidgetObject (Variables|Default|GetHealthBar))))
  (Variables|/Game/UI/WB_HealthBar.WB_HealthBar_C|SetTankRef _aswb_health_bar self))